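; Zacha47 multiplayer gun that players can pick up, throw, aim, reload and fire, configured by a weapon info struct.
; Pickup attaches it to first-person arms locally or third-person body otherwise; throwing restores physics.
; Server-side Use fires line traces, applies game-mode per-bone damage, spends ammo and multicasts effects.
; Spread grows with cooling gun heat and movement speed, dropping to zero while aiming; debug traces and prints remain.
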(event `self.ReceiveTick`
  (params (DeltaSeconds :type "Float (single-precision)"))
  (`self.CoolDown` DeltaSeconds)
  (if (`self.Picked`)
    _))

(event `self.ReceiveBeginPlay`
  (`self.SetMaterial`))

(event `/Game/Data/Interfaces/I_Pickable.Pickup`
  (params (Player :type "/Game/Player/BP_FirstPersonCharacter Object Reference"))
  ;[1 1 1] Pickup / Throw
  (`self.S_Pickup` Player))

(event `S_Pickup`
  (params (OwnerChar :type "/Game/Player/BP_FirstPersonCharacter Object Reference"))
  ;[1 1 1] Pickup / Throw
  (set `self.OwnerChar` OwnerChar)
  (set `self.Picked` true)
  (`self.MC_AttachToOwner`))

(event `MC_AttachToOwner`
  (bind _returnvalue (`GameplayStatics.GetPlayerCharacter` 0))
  (bind _ownerchar (`self.OwnerChar`))
  ;[1 1 1] Pickup / Throw
  (`self.SetPicked` true)
  (if (== _returnvalue _ownerchar)
    (bind _asbp_first_person_character (cast `/Game/Player/BP_FirstPersonCharacter` _returnvalue))
    (bind _asbp_fps_arms (cast `/Game/Player/BP_FPS_Arms` (`ChildActorComponent.ChildActor` (`/Game/Player/BP_FirstPersonCharacter.BP_FPS_Arms` _asbp_first_person_character))))
    (`self.K2_AttachToComponent` (`/Game/Player/BP_FPS_Arms.Zacha47Holder` _asbp_fps_arms) "None" "SnapToTarget" "SnapToTarget" "SnapToTarget")
    (else
      (bind _asbp_third_person_actor (cast `/Game/Player/BP_ThirdPersonActor` (`ChildActorComponent.ChildActor` (`/Game/Player/BP_FirstPersonCharacter.BP_ThirdPersonActor` _ownerchar))))
      (`self.K2_AttachToComponent` (`/Game/Player/BP_ThirdPersonActor.BaseGunHolder` _asbp_third_person_actor) "None" "SnapToTarget" "SnapToTarget" "SnapToTarget"))))

(event `self.ReceiveAnyDamage`
  (params (Damage :type "Float (single-precision)") (DamageType :type "DamageType Object Reference") (InstigatedBy :type "Controller Object Reference") (DamageCauser :type "Actor Object Reference"))
  (`KismetSystemLibrary.PrintString` "Ouch"))

(event `MC_OnShooting`
  ;[1 1 1] On Shooting
  (`ActorComponent.Activate` (`self.P_MuzzleFlash`) true)
  (set `self.GunHeat` (`KismetMathLibrary.FMin` 1.0 (+ (`self.GunHeat`) (`.HeatAddPerShot_39_C6965E194242304892C8EE98E86D5757` (break `/Game/Weapons/STRUCT_WeaponInformation` (`self.Structure`))))))
  (`AudioComponent.Play` (`self.ShootSound`) 0.0))

(event `self.Throw`
  (params (Direction :type "Vector Structure") (Force :type "Float (double-precision)"))
  ;[1 1 1] Pickup / Throw
  (`self.CanThrow`
    (:`Throw`
      (set `self.OwnerChar` null)
      (set `self.Picked` false)
      (`self.MC_Throw` (* Direction Force)))))

(event `MC_Throw`
  (params (Force :type "Vector Structure"))
  ;[1 1 1] Pickup / Throw
  (`self.SetPicked` false)
  (`PrimitiveComponent.AddForce` (`self.SeriousSafetyIssues`) Force "None" false))

(event `self.Use`
  (params (Origin :type "Transform Structure") (Instigator :type "PlayerController Object Reference"))
  (bind ((`BulletPerShot_34_3BFC29F247AB06408C45679B63C1DABB` _bulletpershot) (`RecoilAmtMax_14_427D6B904DA759BD1BFF3D8F3FD6532E` _recoilamtmax) (`ShootSpeed_16_085FB6F640697D89C6B058A790996E91` _shootspeed)) (break `/Game/Weapons/STRUCT_WeaponInformation` (`self.Structure`)))
  ;[1 1 1] Shooting (always on server)
  (`/Engine/EditorBlueprintResources/ActorMacros.Switch Has Authority`
    (:`Authority`
      (bind _usable (`self.CanUse`))
      (if _usable
        (`/Game/Player/BP_FirstPersonCharacter.WeaponShot` (`self.OwnerChar`) _shootspeed _recoilamtmax)
        (for _ (range 1 (+ _bulletpershot 1))
          (`self.Shoot` Origin Instigator))
        (`self.MC_OnShooting`)
        (`self.Add to gun heat`)
        (`self.Remove bullets` 1)
        (else
          (`/Game/Player/BP_FirstPersonCharacter.StopShooting` (`self.OwnerChar`)))))))

(event `self.SphereCollision.OnComponentBeginOverlap`
  (params (OverlappedComponent :type "PrimitiveComponent Object Reference") (OtherActor :type "Actor Object Reference") (OtherComp :type "PrimitiveComponent Object Reference") (OtherBodyIndex :type Integer) (bFromSweep :type Boolean) (SweepResult :type "HitResult Structure (by ref)"))
  (`self.Set Pickup HUD Vis` OtherActor true))

(event `self.SphereCollision.OnComponentEndOverlap`
  (params (OverlappedComponent :type "PrimitiveComponent Object Reference") (OtherActor :type "Actor Object Reference") (OtherComp :type "PrimitiveComponent Object Reference") (OtherBodyIndex :type Integer))
  (`self.Set Pickup HUD Vis` OtherActor))

(event `self.CoolDown`
  (params (DT :type "Float (double-precision)"))
  ;[1 1 1] Shooting (always on server)
  (set `self.GunHeat` (`KismetMathLibrary.FInterpTo` (`self.GunHeat`) 0.0 DT (`.CoolDownSpeed_41_C71F34964A6109FAB756DD8D135DEAB1` (break `/Game/Weapons/STRUCT_WeaponInformation` (`self.Structure`))))))

(event `self.SecondUse`
  (params (Enable :type Boolean))
  ;[1 1 1] Second Action
  (bind _possible (`self.CanSecondUse`))
  (if _possible
    (`self.SetAiming` Enable)))

(event `self.Reload`
  (bind ((`ReloadTime_5_188562684DD64834C94C5FBE030BA66D` _reloadtime) (`ReloadAnim_8_223FBDC64BF7C04B765E2E930C3FF244` _reloadanim)) (break `/Game/Weapons/STRUCT_WeaponInformation` (`self.Structure`)))
  ;[1 1 1] Reload
  (`self.ShouldReload`
    (:`Reload`
      (`/Game/Player/BP_FirstPersonCharacter.PlayReload` (`self.OwnerChar`) _reloadanim)
      (set `self.IsReloading` true)
      (`KismetSystemLibrary.K2_SetTimerDelegate` (delegate `EndReload`) _reloadtime))))

(event `SetAiming`
  (params (IsAiming :type Boolean))
  (bind _ownerchar (`self.OwnerChar`))
  (bind ((`AimHUD_11_75BF687849EAA07DBE4E2388DA1192A6` _aimhud) (`AimFOV_21_5FCEA7274FDDA456B75ED5A4786518DE` _aimfov)) (break `/Game/Weapons/STRUCT_WeaponInformation` (`self.Structure`)))
  ;[1 1 1] Second Action
  (bind _output_get (set `/Game/Player/BP_FirstPersonCharacter.IsAiming` IsAiming _ownerchar))
  (if _output_get
    (`/Game/Player/BP_FirstPersonCharacter.StartAiming` _ownerchar _aimfov _aimhud)
    (else
      (`/Game/Player/BP_FirstPersonCharacter.StopAiming` _ownerchar _aimhud))))

(event `EndReload`
  ;[1 1 1] Reload
  (if (`self.IsReloading`)
    (set `self.IsReloading` false)
    (`self.ReloadAmmo`)))

(fn `Add to gun heat`
  (set `self.GunHeat` (`KismetMathLibrary.FMin` 1.0 (+ (`self.GunHeat`) (`.HeatAddPerShot_39_C6965E194242304892C8EE98E86D5757` (break `/Game/Weapons/STRUCT_WeaponInformation` (`self.Structure`)))))))

(fn `CanSecondUse`
  (returns (Possible :type Boolean))
  (return true))

(fn `CanUse`
  (returns (Usable :type Boolean))
  (return (and (> (`.CurrentAmmo_49_87982919486E5602EA8A8E83EB2903D4` (break `/Game/Weapons/STRUCT_WeaponInformation` (`self.Structure`))) 0) (not (`self.IsReloading`)))))

(fn `Generate Ray Info`
  (params (Origin :type "Transform Structure (by ref)"))
  (returns (Start :type "Vector Structure") (End :type "Vector Structure"))
  (locals (`Ray Length` :type "Float (double-precision)" :default 99000.0))
  (bind _rotation (.rotation Origin))
  (bind _ownerchar (`self.OwnerChar`))
  (bind ((`ShootingSpread_37_A03D94024CBFC0AB4A310B93FE293290` _shootingspread) (`SpreadMaxRunning_43_70C56E8D47C35E6C2700F0B9AF05CC85` _spreadmaxrunning)) (break `/Game/Weapons/STRUCT_WeaponInformation` (`self.Structure`)))
  (bind _charactermovement (`Character.CharacterMovement` _ownerchar))
  (bind _returnvalue (`KismetMathLibrary.SelectFloat` 0.0 1.0 (`/Game/Player/BP_FirstPersonCharacter.IsAiming` _ownerchar)))
  (bind _returnvalue_2 (* _returnvalue (* (`self.GunHeat`) _shootingspread)))
  (bind _returnvalue_3 (+ (* (`KismetMathLibrary.Conv_RotatorToVector` (.rotation Origin)) (`KismetMathLibrary.Conv_DoubleToVector` 100.0)) (.location Origin)))
  (bind _returnvalue_4 (* _returnvalue_2 -1.0))
  (bind _returnvalue_5 (* (* _returnvalue _spreadmaxrunning) (/ (`KismetMathLibrary.VSize` (`CharacterMovementComponent.GetLastUpdateVelocity` _charactermovement)) (`MovementComponent.GetMaxSpeed` _charactermovement))))
  (bind _returnvalue_6 (* _returnvalue_5 -1.0))
  (return _returnvalue_3 (+ (* (`KismetMathLibrary.Conv_DoubleToVector` (`local.Ray Length`)) (`KismetMathLibrary.RotateAngleAxis` (`KismetMathLibrary.RotateAngleAxis` (`KismetMathLibrary.Conv_RotatorToVector` _rotation) (+ (`KismetMathLibrary.RandomFloatInRange` _returnvalue_4 _returnvalue_2) (`KismetMathLibrary.RandomFloatInRange` _returnvalue_6 _returnvalue_5)) (`KismetMathLibrary.GetRightVector` _rotation)) (+ (`KismetMathLibrary.RandomFloatInRange` _returnvalue_4 _returnvalue_2) (`KismetMathLibrary.RandomFloatInRange` _returnvalue_6 _returnvalue_5)) (`KismetMathLibrary.GetUpVector` _rotation))) _returnvalue_3)))

(fn `Get Damage`
  (params (Bone :type Name))
  (returns (Damage_Points :type "Float (double-precision)"))
  (bind _asgm_team_game (cast `/Game/Levels/Game/GM_TeamGame` (`GameplayStatics.GetGameMode`)))
  (bind _damage_points (`/Game/Levels/Game/GM_TeamGame.Get Damage Per Bone` _asgm_team_game Bone))
  (return (* _damage_points (`.DamageBase_45_DFF8045F4E2A0FEDC5F380A5CE1D847C` (break `/Game/Weapons/STRUCT_WeaponInformation` (`self.Structure`))))))

(fn `GetWeaponStruct`
  (returns (Struct :type "/Game/Weapons/STRUCT_WeaponInformation Structure"))
  (return (`self.Structure`)))

(fn `IsPickable`
  (returns (Pickable :type Boolean))
  (return (not (`self.Picked`))))

(fn `ReloadAmmo`
  (bind _structure (`self.Structure`))
  (setmembers `/Game/Weapons/STRUCT_WeaponInformation` :`StructRef` _structure :`CurrentAmmo` (`.MaxAmmo_2_B5D9B2C2447E475F82F48E8EBFB454C8` (break `/Game/Weapons/STRUCT_WeaponInformation` _structure))))

(fn `Remove bullets`
  (params (Amt :type Integer))
  (bind _returnvalue (- (`.CurrentAmmo_49_87982919486E5602EA8A8E83EB2903D4` (break `/Game/Weapons/STRUCT_WeaponInformation` (`self.Structure`))) Amt))
  (setmembers `/Game/Weapons/STRUCT_WeaponInformation` :`StructRef` (`self.Structure`) :`CurrentAmmo` _returnvalue)
  (`KismetSystemLibrary.PrintString` (`KismetStringLibrary.Conv_IntToString` _returnvalue)))

(fn `Set Pickup HUD Vis`
  (params (Actor :type "Object Object Reference") (Visible :type Boolean))
  (bind _aspawn (cast `Pawn` Actor))
  (if (== _aspawn (`GameplayStatics.GetPlayerPawn` 0))
    (`SceneComponent.SetVisibility` (`self.PickupHUD`) (and Visible (not (`self.Picked`))) false)))

(fn `SetMaterial`)

(fn `SetPicked`
  (params (Picked :type Boolean))
  (bind _returnvalue (not Picked))
  (`PrimitiveComponent.SetSimulatePhysics` (`self.SeriousSafetyIssues`) _returnvalue)
  (set `PrimitiveComponent.bGenerateOverlapEvents` _returnvalue (`self.SphereCollision`))
  (`PrimitiveComponent.SetEnableGravity` (`self.SeriousSafetyIssues`) _returnvalue)
  (if Picked
    (`SceneComponent.SetVisibility` (`self.PickupHUD`) false false)
    (`PrimitiveComponent.SetCollisionEnabled` (`self.SphereCollision`) "NoCollision")
    (else
      (`PrimitiveComponent.SetCollisionEnabled` (`self.SphereCollision`) "QueryOnly")))
  (return))

(fn `Shoot`
  (params (Origin :type "Transform Structure (by ref)") (EventInstigator :type "Controller Object Reference"))
  (bind (_start _end) (`self.Generate Ray Info` Origin))
  (bind (_outhit _returnvalue) (`KismetSystemLibrary.LineTraceSingleForObjects` :`Start` _start :`End` _end :`ObjectTypes` (`|MakeArray` "ObjectTypeQuery1" "ObjectTypeQuery2" "ObjectTypeQuery4" "ObjectTypeQuery6" :!type "EObjectTypeQuery Enum") :`DrawDebugType` "Persistent"))
  (if _returnvalue
    (bind (_bblockinghit _binitialoverlap _time _distance _location _impactpoint _normal _impactnormal _physmat _hitactor _hitcomponent _hitbonename) (`GameplayStatics.BreakHitResult` _outhit))
    (if (`KismetMathLibrary.ClassIsChildOf` (`GameplayStatics.GetObjectClass` _hitactor) "/Game/Player/BP_ThirdPersonActor.BP_ThirdPersonActor_C")
      (bind _damage_points (`self.Get Damage` _hitbonename))
      (bind _asbp_first_person_character (cast `/Game/Player/BP_FirstPersonCharacter` (`self.GetParentActor` _hitactor)))
      (`GameplayStatics.ApplyDamage` _asbp_first_person_character _damage_points EventInstigator))))

(fn `UserConstructionScript`)