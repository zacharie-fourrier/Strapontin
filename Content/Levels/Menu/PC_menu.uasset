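; Main menu player controller that shows the main menu UI and starts hosting or joining multiplayer sessions.
; On BeginPlay it loads the settings save and applies the saved player name to the controller and the PS_Menu player state.
; GoToLobby opens the Lobby level as a listen server, and GoToServer joins a given session.
; Both first copy the current player name into FPSGameInstance so it persists across the level change.
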(event `self.ReceiveBeginPlay`
  (bind _returnvalue (`|GenericCreateObject` "/Game/HUD/GUI/Menu/UI_main.UI_main_C"))
  (`UserWidget.AddToViewport` _returnvalue 0)
  (bind _returnvalue_2 (`GameplayStatics.LoadGameFromSlot` "Save"))
  (bind _assave_game_settings (cast `/Game/Data/SaveGame/SaveGameSettings` _returnvalue_2))
  (`self.SetNameTo` (`KismetStringLibrary.Conv_StringToName` (`/Game/Data/SaveGame/SaveGameSettings.PlayerName` _assave_game_settings))))

(event `GoToLobby`
  (`self.Save Name In GameInstance`)
  (`GameplayStatics.OpenLevelBySoftObjectPtr` "/Game/Levels/Lobby/Lobby.Lobby" false "listen"))

(event `GoToServer`
  (params (Session :type "BlueprintSessionResult Structure"))
  (`self.Save Name In GameInstance`)
  (`JoinSessionCallbackProxy.JoinSession` self Session))

(fn `GetName`
  (returns (Name :type Name))
  (return (`KismetStringLibrary.Conv_StringToName` (`AdvancedSessionsLibrary.GetPlayerName` self))))

(fn `Save Name In GameInstance`
  (bind _asfpsgame_instance (cast `/Game/Levels/FPSGameInstance` (`GameplayStatics.GetGameInstance`)))
  (bind _name (`self.GetName`))
  (set `/Game/Levels/FPSGameInstance.SavedGameName` _name _asfpsgame_instance))

(fn `SetNameTo`
  (params (Name :type Name))
  (`AdvancedSessionsLibrary.SetPlayerName` (`GameplayStatics.GetPlayerController` 0) (`KismetStringLibrary.Conv_NameToString` Name))
  (bind _asps_menu (cast `/Game/Levels/Menu/PS_Menu` (`GameplayStatics.GetPlayerState` 0)))
  (set `/Game/Levels/Menu/PS_Menu.Custom Player Name` Name _asps_menu))

(fn `UserConstructionScript`)