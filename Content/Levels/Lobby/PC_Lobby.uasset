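; Lobby player controller that creates the lobby UI and relays lobby and team requests to the game state.
; On BeginPlay it constructs UI_lobby and adds it to the viewport, with no local-controller check.
; Its SendToServer, team-change and team-update events cast the game state to GS_lobby and forward to GSMulticast, ChangeTeam and UpdateTeams respectively.
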(event `self.ReceiveBeginPlay`
  (bind _returnvalue (`|GenericCreateObject` "/Game/Levels/Lobby/UI_lobby.UI_lobby_C"))
  (`UserWidget.AddToViewport` _returnvalue 0))

(event `Send To Server`
  (bind _asgs_lobby (cast `/Game/Levels/Lobby/GS_lobby` (`GameplayStatics.GetGameState`)))
  (`/Game/Levels/Lobby/GS_lobby.GS Multicast` _asgs_lobby))

(event `Send Team Change to Server`
  (params (Player :type "PlayerController Object Reference") (Blue :type "VerticalBox Object Reference") (Orange :type "VerticalBox Object Reference"))
  (bind _asgs_lobby (cast `/Game/Levels/Lobby/GS_lobby` (`GameplayStatics.GetGameState`)))
  (`/Game/Levels/Lobby/GS_lobby.Change Team` _asgs_lobby Player Blue Orange))

(event `Send Update Teams to Server`
  (params (Blue :type "VerticalBox Object Reference") (Orange :type "VerticalBox Object Reference"))
  (bind _asgs_lobby (cast `/Game/Levels/Lobby/GS_lobby` (`GameplayStatics.GetGameState`)))
  (`/Game/Levels/Lobby/GS_lobby.Update Teams` _asgs_lobby Blue Orange))

(fn `UserConstructionScript`)