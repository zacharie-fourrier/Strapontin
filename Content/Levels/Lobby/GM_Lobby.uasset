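; Lobby game mode that admits players to a multiplayer session, balances them into Blue and Orange teams, and launches the match.
; Joiners get a name from the server's local save and the smaller team; logouts leave both lists.
; After a retriggerable delay, players beyond the session's connection limit are kicked and the session updated.
; StartGame copies each team member into the game instance, then server-travels to NewWorld as a listen server.
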(event `self.HandleStartingNewPlayer`
  (params (NewPlayer :type "PlayerController Object Reference"))
  (bind _returnvalue (`GameplayStatics.LoadGameFromSlot` "Save"))
  (bind _assave_game_settings (cast `/Game/Savegame/SaveGameSettings` _returnvalue))
  (`AdvancedSessionsLibrary.SetPlayerName` NewPlayer (`/Game/Savegame/SaveGameSettings.PlayerName` _assave_game_settings))
  (`KismetSystemLibrary.PrintText` (`KismetTextLibrary.Conv_StringToText` (`AdvancedSessionsLibrary.GetPlayerName` NewPlayer)))
  (`self.Assign Player To A team` NewPlayer)
  (`KismetArrayLibrary.Array_AddUnique` (`self.PlayerControllers`) NewPlayer)
  (`KismetSystemLibrary.RetriggerableDelay` 2.0)
  (bind (_numconnections _numprivateconnections _bislan _bisdedicated _ballowinvites _ballowjoininprogress _bisanticheatenabled _builduniqueid _extrasettings) (`AdvancedSessionsLibrary.GetSessionSettings`)
    (:`OnSuccess`
      (if (> (`KismetArrayLibrary.Array_Length` (`GameStateBase.PlayerArray` (`GameplayStatics.GetGameState`))) _numconnections)
        (bind (_arrayindex _arrayelement) (`/Engine/EditorBlueprintResources/StandardMacros.ReverseForEachLoop` (`self.PlayerControllers`))
          (:`LoopBody`
            (if (>= _arrayindex _numconnections)
              (`AdvancedSessionsLibrary.KickPlayer` _arrayelement "Server is Full")))
          (:`Completed`
            (`UpdateSessionCallbackProxyAdvanced.UpdateSession` _extrasettings _numconnections _numprivateconnections)))))))

(event `self.K2_OnLogout`
  (params (ExitingController :type "Controller Object Reference"))
  (bind _asplayer_controller (cast `PlayerController` ExitingController))
  (`KismetArrayLibrary.Array_RemoveItem` (`self.PlayerControllers`) _asplayer_controller)
  (`self.Remove Player From Teams` _asplayer_controller))

(event `Start Game`
  ;[1 0.9234 0] Server traveling
  (bind _asgame_instance_fuck_you (cast `/Game/Data/Variables/GameInstanceFuckYou` (`GameplayStatics.GetGameInstance`)))
  (bind _asgs_lobby (cast `/Game/Levels/Lobby/GS_lobby` (`GameplayStatics.GetGameState`)))
  (for _array_element (`/Game/Levels/Lobby/GS_lobby.Blue Team` _asgs_lobby)
    (`/Game/Data/Variables/GameInstanceFuckYou.AddingPlayer` _asgame_instance_fuck_you (make `/Game/Data/Variables/Player_Info_Struct` (`KismetStringLibrary.Conv_StringToName` (`AdvancedSessionsLibrary.GetPlayerName` _array_element)) 0 0 0 "NewEnumerator1" null _array_element)))
  (for _array_element_2 (`/Game/Levels/Lobby/GS_lobby.Orange Team` _asgs_lobby)
    (`/Game/Data/Variables/GameInstanceFuckYou.AddingPlayer` _asgame_instance_fuck_you (make `/Game/Data/Variables/Player_Info_Struct` (`KismetStringLibrary.Conv_StringToName` (`AdvancedSessionsLibrary.GetPlayerName` _array_element_2)) 0 0 0 "NewEnumerator0" null _array_element_2)))
  (`KismetSystemLibrary.ExecuteConsoleCommand` "ServerTravel NewWorld?Listen" null))

(fn `Assign Player To A team`
  (params (`Joining player` :type "PlayerController Object Reference"))
  (`KismetSystemLibrary.PrintString` "Trying to add a player to the teams")
  (bind _asgs_lobby (cast `/Game/Levels/Lobby/GS_lobby` (`GameplayStatics.GetGameState`)))
  (bind _blue_team (`/Game/Levels/Lobby/GS_lobby.Blue Team` _asgs_lobby))
  (bind _orange_team (`/Game/Levels/Lobby/GS_lobby.Orange Team` _asgs_lobby))
  (if (>= (`KismetArrayLibrary.Array_Length` _blue_team) (`KismetArrayLibrary.Array_Length` _orange_team))
    (`KismetArrayLibrary.Array_AddUnique` _orange_team `Joining player`)
    (else
      (`KismetArrayLibrary.Array_AddUnique` _blue_team `Joining player`)))
  (cast `/Game/Levels/Lobby/GS_lobby` (`GameplayStatics.GetGameState`)))

(fn `Remove Player From Teams`
  (params (`Exiting Player` :type "PlayerController Object Reference"))
  (bind _asgs_lobby (cast `/Game/Levels/Lobby/GS_lobby` (`GameplayStatics.GetGameState`)))
  (`KismetArrayLibrary.Array_RemoveItem` (`/Game/Levels/Lobby/GS_lobby.Blue Team` _asgs_lobby) `Exiting Player`)
  (`KismetArrayLibrary.Array_RemoveItem` (`/Game/Levels/Lobby/GS_lobby.Orange Team` _asgs_lobby) `Exiting Player`)
  (cast `/Game/Levels/Lobby/PC_Lobby` (`GameplayStatics.GetPlayerController` 0)))

(fn `UserConstructionScript`)