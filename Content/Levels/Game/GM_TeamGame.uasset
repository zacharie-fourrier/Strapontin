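; Game mode for a team-based shooter that runs the match from a delayed countdown through team spawns, deaths and a winner announcement.
; It copies team names and timer from URL options into GS_TeamGame, then loops over PC_TeamGame controllers to push countdown, movement locks, killfeed and results.
; New players join positional voice on a shared GUID session, while server Tick updates their speaking state from Vivox.
; Bone damage comes from a data table.
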(event `self.ReceiveTick`
  (params (DeltaSeconds :type "Float (single-precision)"))
  (`/Engine/EditorBlueprintResources/ActorMacros.Switch Has Authority`
    (:`Authority`
      (`self.UpdateSpeaking`))))

(event `DoCountdown`
  ;[1 1 1] Math Timer
  (`self.Start Countdown`)
  (`KismetSystemLibrary.Delay` (`KismetMathLibrary.Conv_IntToDouble` (`self.Countdown Duration`)))
  (`self.Start Match`))

(event `self.ReceiveBeginPlay`
  ;[1 1 1] Begin
  (bind _asfpsgame_instance (cast `/Game/Levels/FPSGameInstance` (`GameplayStatics.GetGameInstance`)))
  (set `self.GI` _asfpsgame_instance)
  (`self.Setup GS Variables`)
  (`KismetSystemLibrary.Delay` 2.0)
  (`self.Call EveryoneLoaded on clients`)
  (`KismetSystemLibrary.Delay` 2.0)
  (`self.DoCountdown`))

(event `Start Match`
  ;[1 1 1] Math Timer
  (`self.StartMatch`)
  (`self.Set Player Movment` true)
  (bind _asgs_team_game (cast `/Game/Levels/Game/GS_TeamGame` (`GameplayStatics.GetGameState`)))
  (`/Game/Levels/Game/GS_TeamGame.Start Timer` _asgs_team_game))

(event `On Player Death`
  (params (PC :type "/Game/Levels/Game/PC_TeamGame Object Reference"))
  ;[1 1 1] Player Rules
  (`/Game/Levels/Game/PC_TeamGame.S_PlayerDied` PC (`self.Respawn Time`) (`self.KeepGunOnDeath`)))

(event `Match End`
  ;[1 1 1] Math Timer
  (`/Engine/EditorBlueprintResources/ActorMacros.Switch Has Authority`
    (:`Authority`
      (`self.EndMatch`)
      (`self.Set Player Movment` false)
      (`self.Match Ended`))))

(event `SpawnPlayer`
  (params (PC :type "/Game/Levels/Game/PC_TeamGame Object Reference"))
  ;[1 1 1] Player Rules
  (`self.Spawn Player in Team Spawn` PC))

(event `self.HandleStartingNewPlayer`
  (params (NewPlayer :type "PlayerController Object Reference"))
  ;[1 1 1] Player Rules
  (bind _aspc_team_game (cast `/Game/Levels/Game/PC_TeamGame` NewPlayer))
  (`self.SpawnPlayer` _aspc_team_game)
  (if (`KismetStringLibrary.IsEmpty` (`self.GameVoiceID`))
    (`self.SetupVoiceID`))
  (`VoicePC.ClientJoinVoice` _aspc_team_game 0 "Positional" (make `SpaceAudioProperties` 4000 200 1.0) (`self.GameVoiceID`))
  (`KismetSystemLibrary.PrintString` (`KismetStringLibrary.Concat_StrStr` "Making " (`AdvancedSessionsLibrary.GetPlayerName` _aspc_team_game) " join the channel " (`self.GameVoiceID`)) true true (struct :`G` 0.66 :`B` 1.0 :`A` 1.0) 30.0))

(fn `Add to clients' killfeed`
  (params (Killer :type "/Game/Levels/Game/PS_TeamGame Object Reference") (Dead :type "/Game/Levels/Game/PS_TeamGame Object Reference"))
  (for _index (range (+ (`GameplayStatics.GetNumPlayerControllers`) 1))
    (bind _aspc_team_game (cast `/Game/Levels/Game/PC_TeamGame` (`GameplayStatics.GetPlayerController` _index)))
    (`/Game/Levels/Game/PC_TeamGame.Killfeed` _aspc_team_game Killer Dead))
  (return))

(fn `Call EveryoneLoaded on clients`
  (for _index (range (+ (`GameplayStatics.GetNumPlayerControllers`) 1))
    (bind _aspc_team_game (cast `/Game/Levels/Game/PC_TeamGame` (`GameplayStatics.GetPlayerController` _index)))
    (`/Game/Levels/Game/PC_TeamGame.OnEveryoneLoaded` _aspc_team_game))
  (return))

(fn `Get Damage Per Bone`
  (params (Bone :type Name))
  (returns (Damage_Points :type "Float (double-precision)"))
  (bind _returnvalue (`|GetDataTableRow` (`self.Damage per bone data`) Bone)
    (:`then`
      (return (`.Damage_Points_5_6E4502514A267C296C691D910204E491` (break `/Game/Data/GameConfig/Transition/Damage_Struct` _returnvalue))))))

(fn `Match Ended`
  (bind _asgs_team_game (cast `/Game/Levels/Game/GS_TeamGame` (`GameplayStatics.GetGameState`)))
  (bind (_name _team _draw) (`/Game/Levels/Game/GS_TeamGame.Get Winning Team` _asgs_team_game))
  (for _index (range (+ (`GameplayStatics.GetNumPlayerControllers`) 1))
    (bind _aspc_team_game (cast `/Game/Levels/Game/PC_TeamGame` (`GameplayStatics.GetPlayerController` _index)))
    (`/Game/Levels/Game/PC_TeamGame.Match Ended` _aspc_team_game _name _team _draw))
  (return))

(fn `Set Player Movment`
  (params (Allowed :type Boolean))
  (for _index (range (+ (`GameplayStatics.GetNumPlayerControllers`) 1))
    (bind _aspc_team_game (cast `/Game/Levels/Game/PC_TeamGame` (`GameplayStatics.GetPlayerController` _index)))
    (set `/Game/Levels/Game/PC_TeamGame.CanMove` Allowed _aspc_team_game))
  (return))

(fn `Setup GS Variables`
  (bind _asgs_team_game (cast `/Game/Levels/Game/GS_TeamGame` (`GameplayStatics.GetGameState`)))
  (set `/Game/Levels/Game/GS_TeamGame.OrangeTeamName` (`GameplayStatics.ParseOption` (`self.OptionsString`) "OTName") _asgs_team_game)
  (set `/Game/Levels/Game/GS_TeamGame.BlueTeamName` (`GameplayStatics.ParseOption` (`self.OptionsString`) "BTName") _asgs_team_game)
  (set `/Game/Levels/Game/GS_TeamGame.TimerSeconds` (`KismetStringLibrary.Conv_StringToInt` (`GameplayStatics.ParseOption` (`self.OptionsString`) "Timer")) _asgs_team_game)
  (return))

(fn `SetupVoiceID`
  (bind _output_get (set `self.GameVoiceID` (`KismetGuidLibrary.Conv_GuidToString` (`KismetGuidLibrary.NewGuid`))))
  (`KismetSystemLibrary.PrintString` (`KismetStringLibrary.Concat_StrStr` "Generated a random GUID for the game: " _output_get) true true (struct :`G` 0.66 :`B` 1.0 :`A` 1.0) 30.0))

(fn `Spawn Player in Team Spawn`
  (params (PC :type "/Game/Levels/Game/PC_TeamGame Object Reference"))
  (bind _team (`/Game/Levels/Game/PC_TeamGame.Get Team` PC))
  (bind _coords (`/Game/Data/GlobalFunctions.Get Respawn Location` _team))
  (`self.RestartPlayerAtTransform` PC (`KismetMathLibrary.MakeTransform` _coords))
  (return))

(fn `Start Countdown`
  (for _index (range (+ (`GameplayStatics.GetNumPlayerControllers`) 1))
    (bind _aspc_team_game (cast `/Game/Levels/Game/PC_TeamGame` (`GameplayStatics.GetPlayerController` _index)))
    (`/Game/Levels/Game/PC_TeamGame.ShowCountdown` _aspc_team_game (`self.Countdown Duration`)))
  (return))

(fn `UpdateSpeaking`
  (bind _gi (`self.GI`))
  (for _index (range (+ (`GameplayStatics.GetNumPlayerControllers`) 1))
    (bind _aspc_team_game (cast `/Game/Levels/Game/PC_TeamGame` (`GameplayStatics.GetPlayerController` _index)))
    (bind _pid (`/Game/Data/GlobalFunctions.Get PID from UNID` (`AdvancedSessionsLibrary.UniqueNetIdToString` (`AdvancedSessionsLibrary.GetUniqueNetID` _aspc_team_game))))
    (`/Game/Levels/Game/PC_TeamGame.UpdateSelfSpeaking` _aspc_team_game (> (`KismetArrayLibrary.Array_Find` (`VoiceGI.GetClientsTalking` _gi (`VoiceGI.GetVivoxChannelName` _gi)) _pid) -1)))
  (return))

(fn `UserConstructionScript`)