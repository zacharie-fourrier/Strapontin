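; Ready Player Me avatar actor that serves as first-person arms attached to the player camera.
; On BeginPlay it optionally runs avatar setup, printing any failure, then attaches to the camera manager, keeping world location and snapping rotation.
; Each Tick it compares the player character's squared velocity to a small threshold and switches the Actions enum on the BP_FP_Arms_Animation instance between moving and near-still states.
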(event `self.ReceiveBeginPlay`
  (if (`self.LoadAvatarOnStart`)
    (`ReadyPlayerMeActorComponent.RunAvatarSetup` (`self.ReadyPlayerMeComponent`) (delegate `OnSetupFailed`)))
  (`self.K2_AttachToActor` (`GameplayStatics.GetPlayerCameraManager` 0) "None" "KeepWorld" "SnapToTarget" "KeepRelative")
  (`KismetSystemLibrary.PrintString` "Done"))

(event `OnSetupFailed`
  (params (errorMessage :type String))
  (`KismetSystemLibrary.PrintString` errorMessage))

(event `self.ReceiveTick`
  (params (DeltaSeconds :type "Float (single-precision)"))
  (bind _returnvalue (`SkeletalMeshComponent.GetAnimInstance` (`self.SkeletalMeshComponent`)))
  (`/Engine/EditorBlueprintResources/StandardMacros.CompareFloat` (`KismetMathLibrary.VSizeSquared` (`self.GetVelocity` (`GameplayStatics.GetPlayerCharacter` 0))) 10.0
    (:`>`
      (bind _asbp_fp_arms_animation (cast `/Game/Characters/Animations/BP_FP_Arms_Animation` _returnvalue))
      (set `/Game/Characters/Animations/BP_FP_Arms_Animation.Actions` "NewEnumerator0" _asbp_fp_arms_animation))
    (:`<`
      (bind _asbp_fp_arms_animation_2 (cast `/Game/Characters/Animations/BP_FP_Arms_Animation` _returnvalue))
      (set `/Game/Characters/Animations/BP_FP_Arms_Animation.Actions` "NewEnumerator1" _asbp_fp_arms_animation_2))))

(event `self.ReceiveHit`
  (params (MyComp :type "PrimitiveComponent Object Reference") (Other :type "Actor Object Reference") (OtherComp :type "PrimitiveComponent Object Reference") (bSelfMoved :type Boolean) (HitLocation :type "Vector Structure") (HitNormal :type "Vector Structure") (NormalImpulse :type "Vector Structure") (Hit :type "HitResult Structure (by ref)")))

(fn `UserConstructionScript`)