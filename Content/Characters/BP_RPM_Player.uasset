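; BP_RPM_Player is a player avatar using a Ready Player Me component, with gun mesh, animation hooks and death and respawn effects.
; It optionally runs avatar setup on start, detecting completion on Tick by comparing the skeletal mesh against a saved reference.
; Events push action, head, recoil and hit values into BP_Player_Animation.
; Death ragdolls the body, plays timed particles with gravity off, then hides it until Respawn restores visibility and collision.
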(event `self.ReceiveBeginPlay`
  (if (`self.LoadAvatarOnStart`)
    (`ReadyPlayerMeActorComponent.RunAvatarSetup` (`self.ReadyPlayerMeComponent`) (delegate `OnSetupFailed`))
    (set `self.Reference Skeletal` (`SkinnedMeshComponent.SkeletalMesh` (`self.SkeletalMeshComponent`)))))

(event `OnSetupFailed`
  (params (errorMessage :type String))
  (`KismetSystemLibrary.PrintString` errorMessage))

(event `Set Animation Action`
  (params (Actions :type "/Game/Characters/Animations/BP_Player_Actions Enum" :default "NewEnumerator1"))
  (bind _asbp_player_animation (cast `/Game/Characters/Animations/BP_Player_Animation` (`SkeletalMeshComponent.GetAnimInstance` (`self.SkeletalMeshComponent`))))
  (set `/Game/Characters/Animations/BP_Player_Animation.Actions` Actions _asbp_player_animation))

(event `Set Head Rotation`
  (params (HeadAngle :type "Float (double-precision)"))
  (bind _asbp_player_animation (cast `/Game/Characters/Animations/BP_Player_Animation` (`SkeletalMeshComponent.GetAnimInstance` (`self.SkeletalMeshComponent`))))
  (set `/Game/Characters/Animations/BP_Player_Animation.HeadAngle` HeadAngle _asbp_player_animation))

(event `Ragdoll`
  (params (bSimulate :type Boolean))
  (bind _skeletalmeshcomponent (`self.SkeletalMeshComponent`))
  ;[1 1 1] Ragdoll
  (`PrimitiveComponent.SetSimulatePhysics` _skeletalmeshcomponent bSimulate)
  (if bSimulate
    (`PrimitiveComponent.WakeAllRigidBodies` _skeletalmeshcomponent)))

(event `PlayRecoil`
  (bind _asbp_player_animation (cast `/Game/Characters/Animations/BP_Player_Animation` (`SkeletalMeshComponent.GetAnimInstance` (`self.SkeletalMeshComponent`))))
  (set `/Game/Characters/Animations/BP_Player_Animation.RecoilAngle` -7.0 _asbp_player_animation))

(event `PlayHit`
  (bind _asbp_player_animation (cast `/Game/Characters/Animations/BP_Player_Animation` (`SkeletalMeshComponent.GetAnimInstance` (`self.SkeletalMeshComponent`))))
  (set `/Game/Characters/Animations/BP_Player_Animation.HitAngle` 15.0 _asbp_player_animation))

(event `self.ReceiveTick`
  (params (DeltaSeconds :type "Float (single-precision)"))
  ;[1 1 1] Update tick
  (`self.CheckLoaded`))

(event `PlayerDies`
  (params (`Respawn Time` :type "Float (single-precision)"))
  ;[1 1 1] Player dies
  (`PrimitiveComponent.SetCollisionProfileName` (`self.SkeletalMeshComponent`) "BlockAll" true)
  (`self.Ragdoll` true)
  (`KismetSystemLibrary.Delay` (`self.WaitBeforeDeathParticles`))
  (`ActorComponent.Activate` (`self.DeathEffect`) true)
  (`SkeletalMeshComponent.SetEnableGravityOnAllBodiesBelow` (`self.SkeletalMeshComponent`) false "None" true)
  (`KismetSystemLibrary.Delay` (`self.WaitAfterDeathParticles`))
  (`SceneComponent.SetVisibility` (`self.SkeletalMeshComponent`) false false)
  (`self.Ragdoll` false)
  (`PrimitiveComponent.SetCollisionEnabled` (`self.SkeletalMeshComponent`) "NoCollision")
  (`SceneComponent.SetVisibility` (`self.SK_FPGun`) false false))

(event `CheckLoaded`
  ;[1 1 1] Check if the avatar loaded and calls the event if it did
  (if (and (and (`self.LoadAvatarOnStart`) (not (== (`self.Reference Skeletal`) (`SkinnedMeshComponent.SkeletalMesh` (`self.SkeletalMeshComponent`))))) (not (`self.IsLoaded`)))
    (`self.AvatarLoads` :!label _label)
    (set `self.IsLoaded` true)
    (elif (and (not (`self.LoadAvatarOnStart`)) (not (`self.IsLoaded`)))
      (goto _label))))

(event `Respawn`
  (params (HasGun :type Boolean))
  ;[1 1 1] Player respawns
  (set `self.IsAlive` true)
  (`ActorComponent.Activate` (`self.RespawnEffect`) true)
  (`SceneComponent.SetVisibility` (`self.SkeletalMeshComponent`) true false)
  (`PrimitiveComponent.SetCollisionEnabled` (`self.SkeletalMeshComponent`) "QueryAndPhysics")
  (`SceneComponent.SetVisibility` (`self.SK_FPGun`) HasGun false)
  (`PrimitiveComponent.SetCollisionProfileName` (`self.SkeletalMeshComponent`) "OverlapAll" true))

(event `AvatarLoads`
  ;[1 1 1] Avatar load
  (`KismetSystemLibrary.PrintString` "Avatar Loaded"))

(fn `UserConstructionScript`)