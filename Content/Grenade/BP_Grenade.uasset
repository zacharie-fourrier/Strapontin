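; Timed grenade actor configured by a data struct for fuse, power, color and sounds, which explodes and damages first-person characters.
; Init starts the fuse timer and a self-rescheduling beep, paced by a curve over remaining fuse time, with emissive flashes decaying on Tick.
; Explosion hides the sphere, plays Niagara and sound, then destroys the actor after a delay.
; Only the server applies inverse-distance damage within a power-sized radius and triggers deaths.
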(event `Init`
  (bind ((`FuseTime_8_F0ACA8894355D90E7B8ADB9C522C853D` _fusetime) (`BeepSound_16_F7FF46E045353CA73C229FAB20A4959F` _beepsound) (`BoomSound_17_F7C68CCA483B02C9CB52C2ACD71B786B` _boomsound)) (break `/Game/Grenade/GrenadeStructure` (`self.Structure`)))
  (`self.StartBeepSounds`)
  (`self.Set material`)
  (`SphereComponent.SetSphereRadius` (`self.ExplosionDetection`) (`.ExplosionPower_5_D22877B041DA5C270F32968ACA952BC8` (break `/Game/Grenade/GrenadeStructure` (`self.Structure`))) true)
  (`KismetSystemLibrary.K2_SetTimerDelegate` (`|CreateDelegate` :!event `Explode`) _fusetime)
  (`self.SetActorTickEnabled` true)
  (`AudioComponent.SetSound` (`self.Beep Sound`) _beepsound)
  (`AudioComponent.SetSound` (`self.ExplosionSound`) _boomsound))

(event `self.ReceiveTick`
  (params (DeltaSeconds :type "Float (single-precision)"))
  (set `self.Time Since Init` (+ DeltaSeconds (`self.Time Since Init`)))
  (`self.UpdateMaterials` DeltaSeconds))

(event `Explode`
  (bind _grenadesphere (`self.GrenadeSphere`))
  (`|ExecutionSequence`
    (:`then_0`
      (set `self.Exploded` true)
      (`self.PlayExplosion`)
      (`SceneComponent.K2_SetWorldRotation` :`self` (`self.GrenadeSphere`))
      (`PrimitiveComponent.SetSimulatePhysics` _grenadesphere false)
      (`PrimitiveComponent.SetCollisionEnabled` _grenadesphere "NoCollision")
      (`ActorComponent.Activate` (`self.Explosion`) false)
      (`SceneComponent.SetVisibility` (`self.GrenadeSphere`) false false)
      (`KismetSystemLibrary.Delay` 2.5)
      (`self.K2_DestroyActor`))
    (:`then_1`
      (if (`KismetSystemLibrary.IsServer`)
        (`self.HurtPlayers`)))))

(event `StartBeepSounds`
  (bind ((`FuseTime_8_F0ACA8894355D90E7B8ADB9C522C853D` _fusetime)) (break `/Game/Grenade/GrenadeStructure` (`self.Structure`)))
  (bind _returnvalue (`CurveFloat.GetFloatValue` (`self.BeepCurve`) (- _fusetime (`self.Time Since Init`))))
  (`self.PlayBeep`)
  (set `self.CurrentEmission` (+ (`self.EmissionBase`) 50.0))
  (if (and (< (+ (`self.Time Since Init`) _returnvalue) _fusetime) (not (`self.Exploded`)))
    (`KismetSystemLibrary.K2_SetTimerDelegate` (`|CreateDelegate` :!event `StartBeepSounds`) _returnvalue)))

(fn `HurtPlayers`
  (bind _explosiondetection (`self.ExplosionDetection`))
  (bind _outactors (`KismetSystemLibrary.ComponentOverlapActors` _explosiondetection (`SceneComponent.K2_GetComponentToWorld` _explosiondetection) (`|MakeArray` "ObjectTypeQuery3" :!type "EObjectTypeQuery Enum") "/Game/FirstPerson/Blueprints/BP_FirstPersonCharacter.BP_FirstPersonCharacter_C"))
  (for _array_element _outactors
    (bind _asbp_first_person_character (cast `/Game/FirstPerson/Blueprints/BP_FirstPersonCharacter` _array_element))
    (`/Game/FirstPerson/Blueprints/BP_FirstPersonCharacter.PlayerHit` _asbp_first_person_character (* (/ (`.ExplosionPower_5_D22877B041DA5C270F32968ACA952BC8` (break `/Game/Grenade/GrenadeStructure` (`self.Structure`))) (`KismetMathLibrary.Vector_Distance` (`self.K2_GetActorLocation` _array_element) (`SceneComponent.K2_GetComponentLocation` (`self.GrenadeSphere`)))) 65.0))
    (`/Game/FirstPerson/Blueprints/BP_FirstPersonCharacter.HitEffect` _asbp_first_person_character)
    (if (and (<= (`/Game/FirstPerson/Blueprints/BP_FirstPersonCharacter.Health` _asbp_first_person_character) 0.0) (`/Game/FirstPerson/Blueprints/BP_FirstPersonCharacter.IsAlive` _asbp_first_person_character))
      (`/Game/FirstPerson/Blueprints/BP_FirstPersonCharacter.Death Client` _asbp_first_person_character)
      (`/Game/FirstPerson/Blueprints/BP_FirstPersonCharacter.PlayerDead` _asbp_first_person_character null))))

(fn `PlayBeep`
  (`AudioComponent.Play` (`self.Beep Sound`) 0.0))

(fn `PlayExplosion`
  (`AudioComponent.Play` (`self.ExplosionSound`) 0.0))

(fn `Set material`
  (bind ((`GrenadeColor_2_94DDD719411528A9A5307AB77E74071D` _grenadecolor) (`ExplosionPower_5_D22877B041DA5C270F32968ACA952BC8` _explosionpower)) (break `/Game/Grenade/GrenadeStructure` (`self.Structure`)))
  (bind _output_get (set `self.EmissionBase` (/ _explosionpower 200.0)))
  (set `self.CurrentEmission` _output_get)
  (`MeshComponent.SetVectorParameterValueOnMaterials` (`self.GrenadeSphere`) "BaseColor" (`KismetMathLibrary.Conv_LinearColorToVector` _grenadecolor))
  (`MeshComponent.SetScalarParameterValueOnMaterials` (`self.GrenadeSphere`) "Emission" (`self.EmissionBase`))
  (`NiagaraComponent.SetVariableLinearColor` (`self.Explosion`) "User.ExplosionColor" _grenadecolor)
  (`NiagaraComponent.SetVariableFloat` (`self.Explosion`) "User.ExplosionPower" _explosionpower))

(fn `UpdateMaterials`
  (params (DeltaTime :type "Float (double-precision)"))
  (bind _output_get (set `self.CurrentEmission` (`KismetMathLibrary.FInterpTo_Constant` (`self.CurrentEmission`) (`self.EmissionBase`) DeltaTime 500.0)))
  (`MeshComponent.SetScalarParameterValueOnMaterials` (`self.GrenadeSphere`) "Emission" _output_get))

(fn `UserConstructionScript`)