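; First-person arms for an FPS player, which can load a Ready Player Me avatar on BeginPlay and print an error if setup fails.
; SetAnimation passes the current Actions to the BP_FP_Arms_Animation instance on the skeletal mesh.
; Anim_Shooting plays a timeline that computes an X-axis recoil offset scaled by RecoilPower.
; The node that would apply that offset to the mesh is unconnected, so this Blueprint never moves it.
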(event `self.ReceiveTick`
  (params (DeltaSeconds :type "Float (single-precision)"))
  ;[1 1 1] Update
)

(event `self.ReceiveBeginPlay`
  ;[1 1 1] Begin
  (if (`self.LoadOnStart`)
    (`ReadyPlayerMeActorComponent.RunAvatarSetup` (`self.ReadyPlayerMeActor`) (delegate `OnSetupFailed`))))

(event `OnSetupFailed`
  (params (errorMessage :type String))
  ;[1 1 1] Begin
  (`KismetSystemLibrary.PrintString` errorMessage true true (struct :`R` 1.0 :`G` 0.045722 :`A` 1.0)))

(event `Anim_Shooting`
  ;[1 1 1] Animations
  (bind (_direction _value) (`Timeline|Shooting Timeline` :!via `PlayFromStart`)
    (:`Update`
      (set `self.RelativeLocation` (`KismetMathLibrary.MakeVector` (+ (* _value (`self.RecoilPower`)) (.x (`KismetMathLibrary.MakeVector` 0.0 0.0 (`.Z` (`KismetMathLibrary.BreakVector3f` (`self.RelativeLocation`)))))) (.y (`KismetMathLibrary.MakeVector` 0.0 0.0 (`.Z` (`KismetMathLibrary.BreakVector3f` (`self.RelativeLocation`))))) (.z (`KismetMathLibrary.MakeVector` 0.0 0.0 (`.Z` (`KismetMathLibrary.BreakVector3f` (`self.RelativeLocation`))))))))))

(fn `SetAnimation`
  (params (Actions :type "/Game/Data/Animations/FP_Arms_actions Enum" :default "NewEnumerator1"))
  (bind _asbp_fp_arms_animation (cast `/Game/Data/Animations/BP_FP_Arms_Animation` (`SkeletalMeshComponent.GetAnimInstance` (`self.SkeletalMesh`))))
  (set `/Game/Data/Animations/BP_FP_Arms_Animation.Actions` Actions _asbp_fp_arms_animation))

(fn `UserConstructionScript`)